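; BP_PawnChariot is a player-controlled paddle pawn that slides sideways and keeps a BP_Pingball in play.
; The Left/Right axis sweeps it along world Y in fixed per-tick steps, unscaled by delta time, with positive input moving toward negative Y.
; On BeginPlay it spawns a ball at SpawnPoint and binds to its OnDeath event, which loops back to spawn and bind a replacement.
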(event Custom|OnDeath_Event
  (bind _output_get (CallFunction|SpawnBall))
  (EventDispatchers|AssignOnDeath _output_get (delegate Custom|OnDeath_Event)))

(event EventBeginPlay
  (bind _output_get (CallFunction|SpawnBall))
  (EventDispatchers|AssignOnDeath _output_get (delegate Custom|OnDeath_Event)))

(event Input|AxisEvents|InputAxisLeft/Right
  (params (AxisValue :type Float%20%28single-precision%29))
  (if (> AxisValue 0.0)
    (Transformation|AddActorWorldOffset "0.000000,-50.000000,0.000000" true)))

(event Input|AxisEvents|InputAxisLeft/Right
  (params (AxisValue :type Float%20%28single-precision%29))
  (if (< AxisValue 0.0)
    (Transformation|AddActorWorldOffset "0.000000,50.000000,0.000000" true)))

(fn ConstructionScript)

(fn SpawnBall
  (bind _returnvalue (Game|SpawnActorfromClass "/Game/Test_grounds/Actors/BP_main_actors/BP_Pingball.BP_Pingball_C" (Math|Transform|MakeTransform (Transformation|GetWorldLocation (Variables|Default|GetSpawn_point)) "0, 0, 0" "1.000000,1.000000,1.000000") "AlwaysSpawn" "MultiplyWithRoot" 0 0))
  (bind _output_get (Variables|Default|SetPlayingBall _returnvalue))
  (return _output_get))