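; BP_PawnChariot_bonuse_Child is a child of a chariot pawn that adds an extra-life bonus reaction to collisions.
; On BeginPlay it has player controller 0 possess it, then runs the parent logic.
; Its Hit event calls the parent, and when the other actor is a BP_ExtraBall_Child, it spawns a BP_Singlelive_Child at the SpawnPoint component's location.
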(event EventBeginPlay
  (Pawn|Possess (Game|GetPlayerController 0) self)
  (|CallParentFunction))

(event Collision|EventHit
  (params (MyComp :type Primitive%20Component%20Object%20Reference) (Other :type Actor%20Object%20Reference) (OtherComp :type Primitive%20Component%20Object%20Reference) (bSelfMoved :type Boolean) (HitLocation :type Vector :default "0, 0, 0") (HitNormal :type Vector :default "0, 0, 0") (NormalImpulse :type Vector :default "0, 0, 0") (Hit :type Hit%20Result%20Structure%20%28by%20ref%29))
  (|CallParentFunction 0 Other 0 false "0, 0, 0" "0, 0, 0" "0, 0, 0" Hit)
  (Utilities|Casting|CastToBP_ExtraBall_Child Other)
  (Game|SpawnActorfromClass "/Game/Test_grounds/Actors/BP_main_actors/Pingball/BP_Single-live_Child.BP_Single-live_Child_C" (Math|Transform|MakeTransform (Transformation|GetWorldLocation (Variables|Default|GetSpawn_point)) "0, 0, 0" "1.000000,1.000000,1.000000") "Undefined" "MultiplyWithRoot" 0 0))

(fn ConstructionScript
  (|CallParentFunction))