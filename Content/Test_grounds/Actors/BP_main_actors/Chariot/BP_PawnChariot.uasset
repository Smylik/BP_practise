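; BP_PawnChariot is a player pawn that slides with sweep along the Left/Right axis and manages the ball and lives in a ball-and-paddle style game.
; On BeginPlay it spawns a BP_Pingball at SpawnPoint and binds its OnDeath.
; Each death spends a life and respawns the ball, or loads MainMenuLevel when none remain.
; Hits with BP_ExtraLive_Child add a life, and life changes update WD_HUD.
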(event Custom|OnDeath_Event
  (if (>= (Variables|Default|GetLives) 1)
    (bind _result (Math|Integer|DecrementInt (Variables|Default|GetLives))
      (:%20%20
        (bind _output_get (Variables|Default|SetLives _result))
        (Variables|/Game/Test_grounds/Widgets/WD_HUD.WD_HUD_C|SetHealth (Utilities|Array|Get(acopy) (stale EventBeginPlay _foundwidgets)) _output_get)
        (bind _output_get_2 (CallFunction|SpawnBall))
        (EventDispatchers|AssignOnDeath _output_get_2 (delegate Custom|OnDeath_Event))))
    (else
      (Game|OpenLevel(byName) "MainMenuLevel"))))

(event EventBeginPlay
  (bind _foundwidgets (Widget|GetAllWidgetsOfClass "/Game/Test_grounds/Widgets/WD_HUD.WD_HUD_C" true))
  (Variables|/Game/Test_grounds/Widgets/WD_HUD.WD_HUD_C|SetHealth (Utilities|Array|Get(acopy) _foundwidgets) (Variables|Default|GetLives))
  (bind _output_get (CallFunction|SpawnBall))
  (EventDispatchers|AssignOnDeath _output_get (delegate Custom|OnDeath_Event)))

(event Collision|EventHit
  (params (MyComp :type Primitive%20Component%20Object%20Reference) (Other :type Actor%20Object%20Reference) (OtherComp :type Primitive%20Component%20Object%20Reference) (bSelfMoved :type Boolean) (HitLocation :type Vector :default "0, 0, 0") (HitNormal :type Vector :default "0, 0, 0") (NormalImpulse :type Vector :default "0, 0, 0") (Hit :type Hit%20Result%20Structure%20%28by%20ref%29))
  (Utilities|Casting|CastToBP_ExtraLive_Child Other)
  (bind _output_get (Variables|Default|SetLives (+ (Variables|Default|GetLives) 1)))
  (Variables|/Game/Test_grounds/Widgets/WD_HUD.WD_HUD_C|SetHealth (Utilities|Array|Get(acopy) (stale EventBeginPlay _foundwidgets)) _output_get))

(event Input|AxisEvents|InputAxisLeft/Right
  (params (AxisValue :type Float%20%28single-precision%29))
  (if (> AxisValue 0.0)
    (Transformation|AddActorWorldOffset (* (* (Variables|Default|GetSpeed) (Variables|Default|GetDirections%201)) (Utilities|Time|GetWorldDeltaSeconds)) true)))

(event Input|AxisEvents|InputAxisLeft/Right
  (params (AxisValue :type Float%20%28single-precision%29))
  (if (< AxisValue 0.0)
    (Transformation|AddActorWorldOffset (* (* (Variables|Default|GetDirections%202) (Variables|Default|GetSpeed)) (Utilities|Time|GetWorldDeltaSeconds)) true)))

(fn ConstructionScript)

(fn SpawnBall
  (bind _returnvalue (Game|SpawnActorfromClass "/Game/Test_grounds/Actors/BP_main_actors/Pingball/BP_Pingball.BP_Pingball_C" (Math|Transform|MakeTransform (Transformation|GetWorldLocation (Variables|Default|GetSpawn_point)) "0, 0, 0" "1.000000,1.000000,1.000000") "AlwaysSpawn" "MultiplyWithRoot" 0 0))
  (bind _output_get (Variables|Default|SetPlayingBall _returnvalue))
  (return _output_get))