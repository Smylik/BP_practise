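; BP_ExtraBall_Child is a child bonus actor, named as an extra-ball pickup, that spawns another actor when hit.
; Its Hit event runs the parent logic, then spawns BP_Singlelive_Child at a spawn transform location, ignoring collisions.
; BeginPlay, overlap and Tick are disabled placeholders, and the construction script only calls the parent.
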(event EventBeginPlay
  (|CallParentFunction) ; This node is disabled and will not be called.\nDrag off pins to build functionality.
)

(event Collision|EventActorBeginOverlap
  (params (OtherActor :type Actor%20Object%20Reference))
  (|CallParentFunction OtherActor) ; This node is disabled and will not be called.\nDrag off pins to build functionality.
)

(event EventTick
  (params (DeltaSeconds :type Float%20%28single-precision%29))
  (|CallParentFunction DeltaSeconds) ; This node is disabled and will not be called.\nDrag off pins to build functionality.
)

(event Collision|EventHit
  (params (MyComp :type Primitive%20Component%20Object%20Reference) (Other :type Actor%20Object%20Reference) (OtherComp :type Primitive%20Component%20Object%20Reference) (bSelfMoved :type Boolean) (HitLocation :type Vector :default "0, 0, 0") (HitNormal :type Vector :default "0, 0, 0") (NormalImpulse :type Vector :default "0, 0, 0") (Hit :type Hit%20Result%20Structure%20%28by%20ref%29))
  (|CallParentFunction 0 Other 0 false "0, 0, 0" "0, 0, 0" "0, 0, 0" Hit)
  (Game|SpawnActorfromClass "/Game/Test_grounds/Actors/BP_main_actors/BP_Single-live_Child.BP_Single-live_Child_C" (Math|Transform|MakeTransform (Variables|Default|GetSpawn%20Transform%20Location) "0, 0, 0" "1.000000,1.000000,1.000000") "AlwaysSpawn" "MultiplyWithRoot" 0 0))

(fn ConstructionScript
  (|CallParentFunction))