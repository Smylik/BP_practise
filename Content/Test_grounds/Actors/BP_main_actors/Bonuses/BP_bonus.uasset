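; BP_bonus is a bonus actor that travels along the world X axis until the player chariot or a kill volume removes it.
; BeginPlay caches the FallBonus component's world location, then each Tick adds SpeedOfFall to X without delta-time scaling and moves the actor with sweep.
; It destroys itself on hitting BP_PawnChariot or overlapping a KillZVolume, with no reward applied in this Blueprint.
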(event Collision|EventHit
  (params (MyComp :type Primitive%20Component%20Object%20Reference) (Other :type Actor%20Object%20Reference) (OtherComp :type Primitive%20Component%20Object%20Reference) (bSelfMoved :type Boolean) (HitLocation :type Vector :default "0, 0, 0") (HitNormal :type Vector :default "0, 0, 0") (NormalImpulse :type Vector :default "0, 0, 0") (Hit :type Hit%20Result%20Structure%20%28by%20ref%29))
  (Utilities|Casting|CastToBP_PawnChariot Other)
  (Actor|DestroyActor))

(event Collision|EventActorBeginOverlap
  (params (OtherActor :type Actor%20Object%20Reference))
  (Utilities|Casting|CastToKillZVolume OtherActor)
  (Actor|DestroyActor))

(event EventTick
  (params (DeltaSeconds :type Float%20%28single-precision%29))
  (bind _starter_location (Variables|Default|GetStarter%20location))
  (bind _output_get (Variables|Default|SetDistance (+ (Variables|Default|GetDistance) (Variables|Default|GetSpeed%20of%20fall))))
  (Transformation|SetActorLocation (Math|Vector|MakeVector _output_get (.y _starter_location) (.z _starter_location)) true false))

(event EventBeginPlay
  (bind _fall_bonus (Variables|Default|Getfall_bonus))
  (bind _returnvalue (Transformation|GetWorldLocation _fall_bonus))
  (Variables|Default|SetStarter%20location (Math|Vector|MakeVector (.x _returnvalue) (.y _returnvalue) (.z _returnvalue)))
  (Variables|Default|SetDistance (.x _returnvalue)))

(fn ConstructionScript)