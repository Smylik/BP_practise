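; BP_Pingball is a bouncing ball actor that moves itself along a direction at its current speed.
; Tick performs a swept world offset and, on a blocking hit, reflects the direction using the surface normal's X and Y.
; The Hit event lowers Speed through Calc while it exceeds MinSpeed, with the step Procentile set from Speed at BeginPlay.
; Overlapping a KillZVolume calls OnDeath and destroys the ball.
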(event EventBeginPlay
  (Variables|Default|SetProcentile (* (Variables|Default|GetSpeed) 0.1)))

(event Collision|EventActorBeginOverlap
  (params (OtherActor :type Actor%20Object%20Reference))
  (Utilities|Casting|CastToKillZVolume OtherActor)
  (Default|CallOnDeath)
  (Actor|DestroyActor))

(event EventTick
  (params (DeltaSeconds :type Float%20%28single-precision%29))
  (bind _sweephitresult (Transformation|AddActorWorldOffset (* (* (Variables|Default|GetDirections) (Variables|Default|GetSpeed)) DeltaSeconds) true))
  (if (.bBlockingHit (Collision|BreakHitResult _sweephitresult))
    (Variables|Default|SetDirections (Math|Vector|GetReflectionVector (Variables|Default|GetDirections) (Math|Vector|MakeVector (.X (Math|Vector|BreakVector (.Normal (Collision|BreakHitResult _sweephitresult)))) (.Y (Math|Vector|BreakVector (.Normal (Collision|BreakHitResult _sweephitresult)))) 0.0)))))

(event Collision|EventHit
  (params (MyComp :type Primitive%20Component%20Object%20Reference) (Other :type Actor%20Object%20Reference) (OtherComp :type Primitive%20Component%20Object%20Reference) (bSelfMoved :type Boolean) (HitLocation :type Vector :default "0, 0, 0") (HitNormal :type Vector :default "0, 0, 0") (NormalImpulse :type Vector :default "0, 0, 0") (Hit :type Hit%20Result%20Structure%20%28by%20ref%29))
  (if (< (Variables|Default|GetMin%20speed) (Variables|Default|GetSpeed))
    (Variables|Default|SetSpeed (|Calc))))

(fn ConstructionScript)