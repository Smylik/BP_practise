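; BP_destruction_changer_Child is a destructible block variant that can drop an extra ball when destroyed.
; On hit, it sets the Block component's material to Red, then passes the hit to the parent's logic.
; On destruction, a 10% weighted random roll spawns BP_ExtraBall_Child at the block's world location.
; Construction only calls the parent script.
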(event EventDestroyed
  (if (Math|Random|RandomBoolwithWeight 0.1)
    (Game|SpawnActorfromClass "/Game/Test_grounds/Actors/BP_main_actors/Bonuses/BP_ExtraBall_Child.BP_ExtraBall_Child_C" (Math|Transform|MakeTransform (Transformation|GetWorldLocation (Variables|Default|GetBlock)) "0, 0, 0" "1.000000,1.000000,1.000000") "Undefined" "MultiplyWithRoot" 0 0)))

(event Collision|EventHit
  (params (MyComp :type Primitive%20Component%20Object%20Reference) (Other :type Actor%20Object%20Reference) (OtherComp :type Primitive%20Component%20Object%20Reference) (bSelfMoved :type Boolean) (HitLocation :type Vector :default "0, 0, 0") (HitNormal :type Vector :default "0, 0, 0") (NormalImpulse :type Vector :default "0, 0, 0") (Hit :type Hit%20Result%20Structure%20%28by%20ref%29))
  (Rendering|Material|SetMaterial (Variables|Default|GetBlock) 0 "/Game/Test_grounds/Primitive_materials/Red.Red")
  (|CallParentFunction 0 Other 0 false "0, 0, 0" "0, 0, 0" "0, 0, 0" Hit))

(fn ConstructionScript
  (|CallParentFunction))