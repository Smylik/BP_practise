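; BP_destruction is a destructible obstacle actor that breaks after taking a set number of hits from BP_Pingball.
; Each Hit event from a pingball decrements the MaxHits counter, which serves as the remaining hit count.
; On the final hit the actor destroys itself, with a small weighted random chance to first spawn a BP_ExtraBall_Child at the Obstacle component's location.
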(event Collision|EventHit
  (params (MyComp :type Primitive%20Component%20Object%20Reference) (Other :type Actor%20Object%20Reference) (OtherComp :type Primitive%20Component%20Object%20Reference) (bSelfMoved :type Boolean) (HitLocation :type Vector :default "0, 0, 0") (HitNormal :type Vector :default "0, 0, 0") (NormalImpulse :type Vector :default "0, 0, 0") (Hit :type Hit%20Result%20Structure%20%28by%20ref%29))
  (Utilities|Casting|CastToBP_Pingball Other)
  (if (<= (Variables|Default|GetMax%20hits) 1)
    (if (Math|Random|RandomBoolwithWeight 0.1)
      (Game|SpawnActorfromClass "/Game/Test_grounds/Actors/BP_main_actors/Bonuses/BP_ExtraBall_Child.BP_ExtraBall_Child_C" (Math|Transform|MakeTransform (Transformation|GetWorldLocation (Variables|Default|GetObstacle)) "0, 0, 0" "1.000000,1.000000,1.000000") "Undefined" "MultiplyWithRoot" 0 0)
      (Actor|DestroyActor)
      (else
        (Actor|DestroyActor)))
    (else
      (Variables|Default|SetMax%20hits (- (Variables|Default|GetMax%20hits) 1)))))

(fn ConstructionScript)